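; BP_Poison is a poison ball that, on impact, becomes a short-lived splat that damages and slows the player.
; On hit the ball is hidden and disabled, the player's max speed is cached, and a line trace positions the splat.
; Timelines grow the splat, then after a delay disable damage, shrink it and destroy the actor.
; Entering the active splat damages once and halves walk speed; leaving restores the cached speed.
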(event OnComponentBeginOverlap(OverlapCollision)
  (params (OverlappedComponent :type Primitive%20Component%20Object%20Reference) (OtherActor :type Actor%20Object%20Reference) (OtherComp :type Primitive%20Component%20Object%20Reference) (OtherBodyIndex :type Integer) (bFromSweep :type Boolean) (SweepResult :type Hit%20Result%20Structure%20%28by%20ref%29))
  (bind _returnvalue (Game|GetPlayerCharacter 0))
  (bind _asfly_swatter_character (Utilities|Casting|CastToFlySwatterCharacter _returnvalue))
  (bind _charactermovement (Variables|/Script/Engine.Character|GetCharacterMovement _asfly_swatter_character))
  (if (and (== OtherActor _returnvalue) (Variables|Default|Getbool%20bCanDamage))
    (Class|FlySwatterCharacter|DamageHealth _asfly_swatter_character)
    (Variables|/Script/Engine.CharacterMovementComponent|SetMaxWalkSpeed _charactermovement (/ (Variables|/Script/Engine.CharacterMovementComponent|GetMaxWalkSpeed _charactermovement) 2.0))))

(event OnComponentEndOverlap(OverlapCollision)
  (params (OverlappedComponent :type Primitive%20Component%20Object%20Reference) (OtherActor :type Actor%20Object%20Reference) (OtherComp :type Primitive%20Component%20Object%20Reference) (OtherBodyIndex :type Integer))
  (if (== OtherActor (Game|GetPlayerCharacter 0))
    (Variables|/Script/Engine.CharacterMovementComponent|SetMaxWalkSpeed (Variables|/Script/Engine.Character|GetCharacterMovement (.AsFly%20Swatter%20Character (Utilities|Casting|CastToFlySwatterCharacter OtherActor))) (Variables|Default|GetCachedSpeed))))

(event OnComponentHit(PoisonBall)
  (params (HitComponent :type Primitive%20Component%20Object%20Reference) (OtherActor :type Actor%20Object%20Reference) (OtherComp :type Primitive%20Component%20Object%20Reference) (NormalImpulse :type Vector :default "0, 0, 0") (Hit :type Hit%20Result%20Structure%20%28by%20ref%29))
  (bind _returnvalue (Class|PoisonSplat|GetPoisonBallMesh))
  (Physics|SetSimulatePhysics _returnvalue false)
  (Collision|SetCollisionEnabled _returnvalue "NoCollision")
  (Rendering|SetVisibility _returnvalue false false)
  (Variables|Default|SetCachedSpeed (Class|MovementComponent|GetMaxSpeed (Variables|/Script/Engine.Character|GetCharacterMovement (.AsFly%20Swatter%20Character (Utilities|Casting|CastToFlySwatterCharacter (Game|GetPlayerCharacter 0))))))
  (Class|PoisonSplat|InitializePoison))

(event EventInitializePoison
  (bind _returnvalue (Class|PoisonSplat|GetSplatMesh))
  (bind _outhit (Collision|LineTraceByChannel (Transformation|GetWorldLocation _returnvalue) (* (Math|Vector|GetUpVector _returnvalue) (Variables|Default|GetGroundCheck)) "TraceTypeQuery1" false 0 "None"))
  (Transformation|SetWorldLocation _returnvalue (.Location (Collision|BreakHitResult _outhit)) false true)
  (Variables|Default|Setbool%20bCanDamage true)
  (bind _alpha (Timeline|ScaleUp Play)
    (:Update
      (Transformation|SetWorldScale3D (Class|PoisonSplat|GetSplatMesh) (Math|Vector|Lerp(Vector) (Transformation|GetWorldScale (Class|PoisonSplat|GetSplatMesh)) (Class|KismetMathLibrary|VectorOne) _alpha)))
    (:Finished
      (Utilities|FlowControl|Delay 1.5)
      (Variables|Default|Setbool%20bCanDamage false)
      (bind _alpha_2 (Timeline|ScaleDown PlayFromStart)
        (:Update
          (Transformation|SetWorldScale3D (Class|PoisonSplat|GetSplatMesh) (Math|Vector|Lerp(Vector) (Transformation|GetWorldScale (Class|PoisonSplat|GetSplatMesh)) "0, 0, 0" _alpha_2)))
        (:Finished
          (Actor|DestroyActor))))))

(fn ConstructionScript)