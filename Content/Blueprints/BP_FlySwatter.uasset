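; Fly swatter actor that homes in on the player character horizontally, keeping its own height.
; BeginPlay caches the player; GoToPlayerLocation plays a timeline that lerps from the current location toward the player's live position each update.
; Within a small tolerance it stops moving and only prints "Smack".
; The random-interval looping timer meant to trigger the move is disconnected, so nothing here starts it.
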(event Custom|Go%20To%20PlayerLocation
  (bind _returnvalue (Transformation|GetActorLocation))
  (bind _returnvalue_2 (Transformation|GetActorLocation))
  (bind _pcharacter (Variables|Default|GetPCharacter))
  (bind _returnvalue_3 (Transformation|GetActorLocation _pcharacter))
  (bind _returnvalue_4 (Math|Vector|MakeVector (.x _returnvalue_3) (.y _returnvalue_3) (.z _returnvalue)))
  (bind _move (Timeline|SmoothMoveTo Play)
    (:Update
      (if (Utilities|Operators|EqualEqual _returnvalue_4 _returnvalue_2 4e+01)
        (Development|PrintString "Smack")
        (else
          (Transformation|SetActorLocation (Math|Vector|Lerp(Vector) _returnvalue_2 _returnvalue_4 _move) false false))))))

(event EventBeginPlay
  (Variables|Default|SetPCharacter (.AsFly%20Swatter%20Character (Utilities|Casting|CastToFlySwatterCharacter (Game|GetPlayerCharacter 0)))))

(fn ConstructionScript)