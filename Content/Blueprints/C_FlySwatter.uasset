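; Fly swatter Blueprint with a hit box that damages the player character on contact.
; The construction script snaps the box to the BoxSocket on the mesh, so it follows that socket.
; Player overlap prints the name and calls DamageHealth on FlySwatterCharacter through a DoOnce, which resets when the overlap ends.
; EnableDamageBox sets BCanDamage, but the overlap logic never checks that flag.
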(event OnComponentBeginOverlap(Box)
  (params (OverlappedComponent :type Primitive%20Component%20Object%20Reference) (OtherActor :type Actor%20Object%20Reference) (OtherComp :type Primitive%20Component%20Object%20Reference) (OtherBodyIndex :type Integer) (bFromSweep :type Boolean) (SweepResult :type Hit%20Result%20Structure%20%28by%20ref%29))
  (bind _returnvalue (Game|GetPlayerCharacter 0))
  (if (== OtherActor _returnvalue)
    (Development|PrintString (Utilities|GetDisplayName OtherActor))
    (Utilities|FlowControl|DoOnce false
      (:Completed
        (Class|FlySwatterCharacter|DamageHealth (.AsFly%20Swatter%20Character (Utilities|Casting|CastToFlySwatterCharacter _returnvalue)))))))

(event OnComponentEndOverlap(Box)
  (params (OverlappedComponent :type Primitive%20Component%20Object%20Reference) (OtherActor :type Actor%20Object%20Reference) (OtherComp :type Primitive%20Component%20Object%20Reference) (OtherBodyIndex :type Integer))
  (bind _returnvalue (Game|GetPlayerCharacter 0))
  (if (== OtherActor _returnvalue)
    (Utilities|FlowControl|DoOnce false) ; enters at Reset
  ))

(event Custom|EnableDamageBox
  (params (Enable :type Boolean))
  (Variables|Default|SetBCanDamage Enable))

(fn ConstructionScript
  (Transformation|AttachComponentToComponent (Variables|Default|GetBox) (Variables|Character|GetMesh) "BoxSocket" "SnapToTarget" "KeepRelative" "KeepRelative" true))